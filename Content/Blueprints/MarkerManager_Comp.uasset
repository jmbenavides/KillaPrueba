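; Marker manager component that shows screen-space widgets over the actors that created them.
; StoreMarkers registers each marker once and adds its MarkerType and CircleIndicator widgets to the viewport.
; Tick projects each valid creator's location for player 0, moving MarkerType there when on screen and hiding it otherwise.
; CircleIndicator is never updated here, and UbicateMarkers is an empty stub.
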(event EventBeginPlay)

(event EventTick
  (params (DeltaSeconds :type Float%20%28single-precision%29))
  (bind _arrayelement (Utilities|Array|ReverseforEachLoop (Variables|Default|GetMarkers))
    (:LoopBody
      (Utilities|IsValid (.MarkerCreator (Utilities|Struct|BreakSTR_Markables _arrayelement))
        (:Is%20Valid
          (CallFunction|UpdateMarkers _arrayelement))))))

(fn StoreMarkers
  (params (Marker :type STR%20Markables%20Structure))
  (bind (_markertype _circleindicator) (Utilities|Struct|BreakSTR_Markables Marker))
  (if (not (Utilities|Array|ContainsItem (Variables|Default|GetMarkers) Marker))
    (Utilities|Array|AddUnique (Variables|Default|GetMarkers) Marker)
    (UserInterface|Viewport|AddtoViewport _markertype 0)
    (UserInterface|Viewport|AddtoViewport _circleindicator 0)))

(fn UbicateMarkers
  (params (Marker :type STR%20Markables%20Structure)))

(fn UpdateMarkers
  (params (Marker :type STR%20Markables%20Structure))
  (bind _markertype (Utilities|Struct|BreakSTR_Markables Marker))
  (bind (_inscreen _screenlocation) (CallFunction|InScreen? Marker))
  (if _inscreen
    (Widget|SetVisibility _markertype "HitTestInvisible")
    (Class|UserWidget|SetPositioninViewport _markertype _screenlocation true)
    (else
      (Widget|SetVisibility _markertype "Hidden"))))

(fn InScreen?
  (params (MarkerLocation :type STR%20Markables%20Structure))
  (bind _markercreator (Utilities|Struct|BreakSTR_Markables MarkerLocation))
  (bind _returnvalue (Game|GetPlayerController 0))
  (bind _returnvalue_2 (Game|GetPlayerController 0))
  (bind _returnvalue_3 (Transformation|GetActorLocation _markercreator))
  (bind (_sizex _sizey) (HUD|GetViewportSize _returnvalue_2))
  (bind (_screenposition _returnvalue_4) (Class|GameplayStatics|ProjectWorldtoScreen _returnvalue _returnvalue_3 false))
  (bind (_x _y) (Math|Vector2D|BreakVector2D _screenposition))
  (return (Math|Boolean|ANDBoolean (>= _x 0.0) (>= _y 0.0) (< _x (Math|Conversions|ToFloat(Integer) _sizex)) (< _y (Math|Conversions|ToFloat(Integer) _sizey)) _returnvalue_4) _screenposition))