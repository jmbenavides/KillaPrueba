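; BP_Markable is an actor that gives itself on-screen marker widgets and registers them with the game's marker manager.
; On BeginPlay, InitMaker creates a marker of the configurable MarkerType class and a WID_CircleIndicator for player 0, passing each a reference to the actor.
; It then stores both widgets and itself as an STRMarkables struct in the MarkerManager_Comp on GameModePrueba.
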(event EventBeginPlay
  (CallFunction|InitMaker))

(event Collision|EventActorBeginOverlap
  (params (OtherActor :type Actor%20Object%20Reference)))

(fn ConstructionScript)

(fn InitMaker
  (Utilities|FlowControl|Sequence
    (:then_0
      (bind _returnvalue (UserInterface|CreateWidget (Variables|Marker|GetMarkerType) (Game|GetPlayerController 0)))
      (bind _output_get (LocalVariables|SetMarker _returnvalue))
      (Class|MarkerInterface|SetCreator(Message) _output_get self))
    (:then_1
      (bind _returnvalue_2 (UserInterface|CreateWidget "/Game/Blueprints/WID_CircleIndicator.WID_CircleIndicator_C" (Game|GetPlayerController 0)))
      (bind _output_get_2 (LocalVariables|SetCircleIndicator _returnvalue_2))
      (Class|MarkerInterface|SetCreator(Message) _output_get_2 self))
    (:then_2
      (bind _asgame_mode_prueba (Utilities|Casting|CastToGameModePrueba (Game|GetGameMode)))
      (Default|StoreMarkers (Actor|GetComponentbyClass _asgame_mode_prueba "/Game/Blueprints/MarkerManager_Comp.MarkerManager_Comp_C") (Utilities|Struct|MakeSTR_Markables (LocalVariables|GetMarker) (LocalVariables|GetCircleIndicator) self)))))